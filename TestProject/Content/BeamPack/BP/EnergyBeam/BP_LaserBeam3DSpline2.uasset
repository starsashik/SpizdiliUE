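; Laser beam actor that sweeps on a timeline-driven rotation and stretches a 3D beam mesh to whatever it hits.
; The construction script builds Z-forward spline meshes along the spline, keeping the last as NewMesh.
; Each tick, a forward trace from Point moves the spline end and mesh, and drives the beam and impact effects, deactivating both effects on a miss.
; Fire decal spawning is present but unconnected.
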(event EventTick
  (params (DeltaSeconds :type Float%20%28single-precision%29))
  (bind _point (Variables|Default|GetPoint))
  (bind _spline (Variables|Default|GetSpline))
  (bind _spline_2 (Variables|Default|GetSpline))
  (bind _spline_3 (Variables|Default|GetSpline))
  (bind _hit (Variables|Default|GetHit))
  (bind _spline_4 (Variables|Default|GetSpline))
  (bind _returnvalue (Transformation|GetWorldRotation _point))
  (bind _returnvalue_2 (Transformation|GetWorldLocation _point))
  (bind _returnvalue_3 (Math|Vector|GetForwardVector _returnvalue))
  (bind _returnvalue_4 (* _returnvalue_3 1e+04))
  (bind _returnvalue_5 (+ _returnvalue_2 _returnvalue_4))
  (bind _outhit (Collision|LineTraceByChannel _returnvalue_2 _returnvalue_5 "TraceTypeQuery1" true 0 "None"))
  (if (.bBlockingHit (Collision|BreakHitResult _outhit))
    (Components|Activation|SetActive (Variables|Default|GetHit) true false)
    (Utilities|FlowControl|Sequence
      (:then_0
        (Transformation|SetWorldRotation _hit (Math|Conversions|RotationFromXVector (.Normal (Collision|BreakHitResult _outhit))) false false)
        (Transformation|SetWorldLocation _hit (+ (.Location (Collision|BreakHitResult _outhit)) 10) false false))
      (:then_1
        (Effects|Components|ParticleSystem|SetVectorParameter (Variables|Default|GetLaserBeam) "Beam End" (.Location (Collision|BreakHitResult _outhit))))
      (:then_2
        (Spline|SetLocationatSplinePoint (Variables|Default|GetSpline) 1 (.Location (Collision|BreakHitResult _outhit)) "World" true)
        (SplineMesh|SetStartandEnd (Variables|Default|GetNewMesh) (Spline|GetLocationatSplinePoint _spline 0 "Local") (Spline|GetTangentatSplinePoint _spline 0 "Local") (Spline|GetLocationatSplinePoint _spline_2 1 "Local") (Spline|GetTangentatSplinePoint _spline_2 1 "Local") true :!class /Script/Engine.SplineMeshComponent)))
    (else
      (Components|Activation|SetActive (Variables|Default|GetHit) false false)
      (Spline|SetLocationatSplinePoint (Variables|Default|GetSpline) 1 _returnvalue_5 "World" true)
      (SplineMesh|SetStartandEnd (Variables|Default|GetNewMesh) (Spline|GetLocationatSplinePoint _spline_3 0 "Local") (Spline|GetTangentatSplinePoint _spline_3 0 "Local") (Spline|GetLocationatSplinePoint _spline_4 1 "Local") (Spline|GetTangentatSplinePoint _spline_4 1 "Local") true :!class /Script/Engine.SplineMeshComponent))))

(event EventBeginPlay
  (bind _defaultsceneroot (Variables|Default|GetDefaultSceneRoot))
  (bind _returnvalue (Transformation|GetWorldRotation _defaultsceneroot))
  (bind (_direction _rotex _zrot) (Timeline|RotateLaser PlayFromStart)
    (:Update
      (Transformation|SetWorldRotation _defaultsceneroot (Math|Rotator|MakeRotator (* _zrot 2e+01) (- _rotex (.roll _returnvalue)) (.yaw _returnvalue)) false false))))

(fn ConstructionScript
  (bind _spline (Variables|Default|GetSpline))
  (bind _spline_2 (Variables|Default|GetSpline))
  (for _index (range 0 (- (Spline|GetNumberOfSplinePoints (Variables|Default|GetSpline)) 2))
    (bind _returnvalue (AddComponent|AddSplineMeshComponent false))
    (bind _output_get (Variables|Default|SetNewMesh _returnvalue))
    (SplineMesh|SetForwardAxis _output_get "Z" true)
    (SplineMesh|SetStartandEnd _output_get (Spline|GetLocationatSplinePoint _spline _index "Local") (Spline|GetTangentatSplinePoint _spline 0 "Local") (Spline|GetLocationatSplinePoint _spline_2 (+ _index 1) "Local") (Spline|GetTangentatSplinePoint _spline_2 (+ _index 1) "Local") true :!class /Script/Engine.SplineMeshComponent)))